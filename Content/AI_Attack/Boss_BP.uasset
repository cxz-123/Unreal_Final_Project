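; Boss enemy Blueprint that chases the player, performs melee montage attacks and shows a world-space health bar.
; A looping timer attacks when off cooldown and in range, or focuses and moves toward the player during cooldown.
; An Attacks flag blocks decisions until the montage ends; the random pick only yields one montage, leaving the others unwired.
; Tick yaws the bar toward the camera and updates its percentage.
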(event `self.ReceiveBeginPlay`
  (`|ExecutionSequence`
    (:`then_0`
      (bind _returnvalue (`KismetSystemLibrary.K2_SetTimerDelegate` (delegate `OB`) 0.1 true :!label _label)))
    (:`then_1`
      (`self.Get_Progress_Bar`))))

(event `OB`
  (bind _returnvalue (`GameplayStatics.GetPlayerCharacter` 0))
  (if (`self.Attacks`)
    _
    (elif (> (- (`GameplayStatics.GetTimeSeconds`) (`self.Attack_Last_Time`)) (`self.Attack_CD`))
      (if (<= (`self.GetDistanceTo` self _returnvalue) 250.0)
        (set `self.Attack_Last_Time` (`GameplayStatics.GetTimeSeconds`))
        (`self.Attack`))
      (else
        (`AIController.K2_SetFocus` (`AIBlueprintHelperLibrary.GetAIController` (`self.GetController` self)) _returnvalue)
        (`|AIMoveTo` self (0.0 0.0 0.0) (`GameplayStatics.GetPlayerCharacter` 0) 100.0 true
          (:`then`
            (`KismetSystemLibrary.K2_ClearAndInvalidateTimerHandle` (stale `self.ReceiveBeginPlay` _returnvalue))
            (`KismetSystemLibrary.Delay` 0.2)
            (goto _label)))))))

(event `Attack`
  (bind _returnvalue (`KismetMathLibrary.RandomIntegerInRange` 0))
  (set `self.Attacks` true)
  (`KismetSystemLibrary.PrintString` (`KismetStringLibrary.Conv_IntToString` _returnvalue))
  (switch `int` _returnvalue
    (:`0`
      (set `self.Montage` "/Game/AI_Attack/Montage/Twinblades_attack02_Montage.Twinblades_attack02_Montage")
      (bind _returnvalue_2 (`self.PlayAnimMontage` self (`self.Montage`) 1.0 "None"))
      (`KismetSystemLibrary.Delay` _returnvalue_2)
      (set `self.Attacks` false)
      (`KismetSystemLibrary.PrintString` "Hello"))))

(event `self.ReceiveTick`
  (params (DeltaSeconds :type "Float (single-precision)"))
  (`self.HP_Bar_LookAtCamera`)
  (`ProgressBar.SetPercent` (`self.Progress_Bar`) (`self.Health_Percent`)))

(fn `Get_Progress_Bar`
  (bind _ashealth_boss_ui (cast `/Game/AI_Attack/Boss_UI/Health_Boss_UI` (`WidgetComponent.GetUserWidgetObject` (`self.Widget`))))
  (set `self.Progress_Bar` (`/Game/AI_Attack/Boss_UI/Health_Boss_UI.ProgressBar_599` _ashealth_boss_ui)))

(fn `HP_Bar_LookAtCamera`
  (bind _widget (`self.Widget`))
  (`SceneComponent.K2_SetWorldRotation` _widget (`KismetMathLibrary.MakeRotator` (.roll (`SceneComponent.K2_GetComponentRotation` _widget)) (.pitch (`SceneComponent.K2_GetComponentRotation` _widget)) (+ (.yaw (`self.K2_GetActorRotation` (`GameplayStatics.GetPlayerCameraManager` 0))) 180.0)) false false))

(fn `UserConstructionScript`)